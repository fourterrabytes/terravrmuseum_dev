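; BP_ArtpieceFocusPoint is a trigger that plays audio commentary with subtitles for an artpiece.
; On box overlap, gated by a DoOnce, it plays the first commentary sound in 2D and prints its name.
; It creates a subtitle widget with the first subtitle entry, sets it on the VRPawn's widget component and also adds it to the viewport.
; After a fixed delay it clears the component's widget and re-arms the DoOnce.
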(event OnComponentBeginOverlap(Box)
  (params (OverlappedComponent :type Primitive%20Component%20Object%20Reference) (OtherActor :type Actor%20Object%20Reference) (OtherComp :type Primitive%20Component%20Object%20Reference) (OtherBodyIndex :type Integer) (bFromSweep :type Boolean) (SweepResult :type Hit%20Result%20Structure%20%28by%20ref%29))
  (bind _audiocommentarysoundclips (Variables|AudioComm|GetAudioCommentarySoundClips))
  (bind _output (Utilities|Array|Get(acopy) _audiocommentarysoundclips))
  (Utilities|FlowControl|DoOnce false :!label _label
    (:Completed
      (Development|PrintString (Utilities|GetDisplayName _output))
      (Audio|PlaySound2D _output 1.0 1.0 0.0 0 0)
      (bind _asvrpawn (Utilities|Casting|CastToVRPawn (Game|Player|GetPlayerPawn 0)))
      (bind _returnvalue (UserInterface|CreateWidget "/Game/UIUX/PlayerUI/UI_AudioTextSubtitles.UI_AudioTextSubtitles_C" (Game|GetPlayerController 0)))
      (UserInterface|SetWidget (Variables|/Game/VRTemplate/Blueprints/VRPawn.VRPawn_C|GetAudioTextSubtitles _asvrpawn) _returnvalue)
      (Default|SetText _returnvalue (Utilities|Array|Get(acopy) (Variables|AudioComm|GetAudioCommentarySubtitles)))
      (UserInterface|Viewport|AddtoViewport _returnvalue 0)
      (Utilities|FlowControl|Delay 1e+01)
      (UserInterface|SetWidget (Variables|/Game/VRTemplate/Blueprints/VRPawn.VRPawn_C|GetAudioTextSubtitles _asvrpawn) 0)
      (goto _label Reset))))

(event EventBeginPlay)

(event Collision|EventActorBeginOverlap
  (params (OtherActor :type Actor%20Object%20Reference)))

(event EventTick
  (params (DeltaSeconds :type Float%20%28single-precision%29)))

(fn ConstructionScript)