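; Teleporter node actor that moves the player to another level when the VR pawn touches its collision component.
; On overlap it prints the component's name and identifies the pawn's sphere by a hardcoded display-name prefix rather than a cast.
; A match plays a fade widget's animation in reverse and starts a timer that then opens the target level.
; The construction script labels the teleporter's text with the destination level name.
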(event OnComponentBeginOverlap(TeleporterCollision)
  (params (OverlappedComponent :type Primitive%20Component%20Object%20Reference) (OtherActor :type Actor%20Object%20Reference) (OtherComp :type Primitive%20Component%20Object%20Reference) (OtherBodyIndex :type Integer) (bFromSweep :type Boolean) (SweepResult :type Hit%20Result%20Structure%20%28by%20ref%29))
  (bind _returnvalue (Utilities|GetDisplayName OtherComp))
  (Development|PrintString _returnvalue true true "(R=0.000000,G=0.660000,B=1.000000,A=1.000000)" 2e+01)
  (if (Utilities|Enum|Equal(Enum) (Utilities|String|GetSubstring _returnvalue 0 17) "VRPawn_C_0.Sphere")
    (bind _returnvalue_2 (UserInterface|CreateWidget "/Game/UIUX/PlayerUI/UI_FadeOut.UI_FadeOut_C" (Game|GetPlayerController 0)))
    (UserInterface|Viewport|AddtoViewport _returnvalue_2 0)
    (UserInterface|Animation|PlayAnimation _returnvalue_2 (Variables|/Game/UIUX/PlayerUI/UI_FadeOut.UI_FadeOut_C|GetfadeAnim _returnvalue_2) 0.0 1 "Reverse" 1.0 false)
    (Utilities|Time|SetTimerbyEvent (delegate Custom|moveToNewExhibit) 3.0)))

(event Custom|moveToNewExhibit
  (Game|OpenLevel(byObjectReference) (Variables|Default|GetLevelToTeleport)))

(event EventBeginPlay)

(event Collision|EventActorBeginOverlap
  (params (OtherActor :type Actor%20Object%20Reference)))

(event EventTick
  (params (DeltaSeconds :type Float%20%28single-precision%29)))

(fn ConstructionScript
  (Rendering|Components|TextRender|SetText (Variables|Default|GetTextRender) (Utilities|Text|ToText(String) (Utilities|String|Append "Teleporter to  
" (Variables|Default|GetLevelName)))))