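; ExitNode is a maze exit actor that advances the player to the next floor.
; When the player character overlaps its Collider, it increments FloorCount on the GameInstanceReal game instance, which persists across level loads.
; It then reopens the EM_MazeLevel map by object reference and prints the new floor count for debugging.
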(event OnComponentBeginOverlap(Collider)
  (params (OverlappedComponent :type Primitive%20Component%20Object%20Reference) (OtherActor :type Actor%20Object%20Reference) (OtherComp :type Primitive%20Component%20Object%20Reference) (OtherBodyIndex :type Integer) (bFromSweep :type Boolean) (SweepResult :type Hit%20Result%20Structure%20%28by%20ref%29))
  (if (== OtherActor (Game|GetPlayerCharacter 0))
    (bind _asgame_instance_real (Utilities|Casting|CastToGameInstanceReal (Game|GetGameInstance)))
    (bind _result (Math|Integer|IncrementInt (Variables|/Game/Blueprints/General/GameInstanceReal.GameInstanceReal_C|GetfloorCount _asgame_instance_real))
      (:%20%20
        (bind _output_get (Variables|/Game/Blueprints/General/GameInstanceReal.GameInstanceReal_C|SetfloorCount _asgame_instance_real _result))
        (Game|OpenLevel(byObjectReference) "/Game/ThirdPerson/Maps/EM_MazeLevel.EM_MazeLevel")
        (Development|PrintString (Utilities|String|ToString(Integer) _output_get))))))

(event EventBeginPlay)

(event Collision|EventActorBeginOverlap
  (params (OtherActor :type Actor%20Object%20Reference)))

(event EventTick
  (params (DeltaSeconds :type Float%20%28single-precision%29)))

(fn ConstructionScript)