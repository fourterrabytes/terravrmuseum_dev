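; Interactable power breaker box that the player opens and switches on to restore the level's power.
; Interact swings the hinged door via timeline and, on alternate uses once open, hides the player mesh and blends the view to the breaker with mouse clicking enabled.
; Clicking the switch sets game mode PowerOn, rotates it and restores the player view.
; The rotation timeline's Update also triggers a flicker sequence, cabinet material swap and lighting changes.
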(event OnClicked(powerButton)
  (params (TouchedComponent :type Primitive%20Component%20Object%20Reference) (ButtonPressed :type Key%20Structure))
  (bind _returnvalue (Game|GetPlayerController 0))
  (bind _asbpem_dev_game_mode (Utilities|Casting|CastToBPEM_devGameMode (Game|GetGameMode)))
  (if (not (Variables|/Game/BPEM_devGameMode.BPEM_devGameMode_C|GetpowerOn? _asbpem_dev_game_mode))
    (Variables|/Game/BPEM_devGameMode.BPEM_devGameMode_C|SetpowerOn? _asbpem_dev_game_mode true)
    (bind _rotateval (Timeline|rotator Play)
      (:Update
        (Transformation|SetRelativeRotation (Variables|Default|GetpowerButton) (Math|Rotator|MakeRotator 0.0 0.0 _rotateval) false false)
        (bind _asbp_tpchar (Utilities|Casting|CastToBP_TPChar (Game|GetPlayerCharacter 0)))
        (Default|SetMeshVisibility _asbp_tpchar true)
        (Game|Player|SetViewTargetwithBlend _returnvalue _asbp_tpchar 1.0 "VTBlend_Linear" 0.0 false)
        (Variables|/Script/Engine.PlayerController|SetbShowMouseCursor _returnvalue false)
        (Variables|/Script/Engine.PlayerController|SetbEnableClickEvents _returnvalue false)
        (bind _outactor (Sequencer|Player|CreateLevelSequencePlayer "/Game/CInematics/EM_flicker.EM_flicker"))
        (Sequencer|Player|Play (Variables|/Script/LevelSequence.LevelSequenceActor|GetSequencePlayer _outactor) :!class /Script/MovieScene.MovieSceneSequencePlayer)
        (Utilities|FlowControl|Delay 5.0)
        (Sequencer|Player|Stop (Variables|/Script/LevelSequence.LevelSequenceActor|GetSequencePlayer _outactor) :!class /Script/MovieScene.MovieSceneSequencePlayer)
        (bind _outactors (Actor|GetAllActorsOfClass "/Game/Blueprints/RealWorld/BP_EMcabinet.BP_EMcabinet_C"))
        (Default|CallSetMaterialsAfterPoweron (Utilities|Array|Get(acopy) _outactors))
        (bind _outactors_2 (Actor|GetAllActorsOfClass "/Game/Blueprints/RealWorld/BP_FlickeringLight.BP_FlickeringLight_C"))
        (for _array_element _outactors_2
          (Rendering|SetVisibility (Variables|/Game/Blueprints/RealWorld/BP_FlickeringLight.BP_FlickeringLight_C|GetflickLight _array_element) false false)
          (bind _outactors_3 (Actor|GetAllActorsOfClass "/Game/Blueprints/RealWorld/BP_FloodLight.BP_FloodLight_C"))
          (for _array_element_2 _outactors_3
            (Rendering|Components|Light|SetIntensity (Variables|/Game/Blueprints/RealWorld/BP_FloodLight.BP_FloodLight_C|GetmainLight _array_element_2) 1e+04)))))))

(event Custom|swingDoorOpen
  (bind _degreeval (Timeline|swingOpen Play)
    (:Update
      (Transformation|SetRelativeRotation (Variables|Default|Gethinge) (Math|Rotator|MakeRotator 0.0 0.0 _degreeval) false false))
    (:Finished
      (Variables|Default|SetdoorOpen true))))

(event Custom|goToPowerSwitch
  (bind _returnvalue (Game|GetPlayerController 0))
  (Utilities|FlowControl|FlipFlop
    (:A
      (if (Variables|Default|GetdoorOpen)
        (bind _asbp_tpchar (Utilities|Casting|CastToBP_TPChar (Game|GetPlayerCharacter 0)))
        (Default|SetMeshVisibility _asbp_tpchar false)
        (Game|Player|SetViewTargetwithBlend _returnvalue self 1.0 "VTBlend_Linear" 0.0 false)
        (Variables|/Script/Engine.PlayerController|SetbShowMouseCursor _returnvalue true)
        (Variables|/Script/Engine.PlayerController|SetbEnableClickEvents _returnvalue true)))))

(event EventBeginPlay)

(event Collision|EventActorBeginOverlap
  (params (OtherActor :type Actor%20Object%20Reference)))

(event EventTick
  (params (DeltaSeconds :type Float%20%28single-precision%29)))

(fn ConstructionScript
  (|CallParentFunction))

(fn Interact
  (params (InteractingActor :type Character%20Object%20Reference))
  (CallFunction|SwingDoorOpen)
  (CallFunction|GotoPowerSwitch)
  (return false 0))