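; BP_Art2DVideoTemplate is a template actor for displaying a 2D art piece with an information placard, configured per instance.
; The construction script creates a dynamic material from VideoMaterial, feeds it the image plus normal, specular and ambient occlusion textures, and scales the mesh's Y axis to the image's aspect ratio.
; On BeginPlay, it creates a UI_Placard widget, fills in the artist, title, description, dimensions and materials, and assigns it to PlacardText.
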(event EventBeginPlay
  (|CallParentFunction)
  ;[1 1 1] setting placard text
  (bind _returnvalue (UserInterface|CreateWidget "/Game/UIUX/MuseumUI/UI_Placard.UI_Placard_C" (Game|GetPlayerController 0)))
  (Variables|/Game/UIUX/MuseumUI/UI_Placard.UI_Placard_C|SetArtistNameText _returnvalue (Variables|PlacardValues|GetartistNameVal))
  (Variables|/Game/UIUX/MuseumUI/UI_Placard.UI_Placard_C|SetArtNameText _returnvalue (Variables|PlacardValues|GetartNameVal))
  (Variables|/Game/UIUX/MuseumUI/UI_Placard.UI_Placard_C|SetDescriptText _returnvalue (Variables|PlacardValues|GetartDescriptionVal))
  (Variables|/Game/UIUX/MuseumUI/UI_Placard.UI_Placard_C|SetDimensionsText _returnvalue (Variables|PlacardValues|GetdimensionVal))
  (Variables|/Game/UIUX/MuseumUI/UI_Placard.UI_Placard_C|SetMaterialText _returnvalue (Variables|PlacardValues|GetmaterialsVal))
  (UserInterface|SetWidget (Variables|Default|GetPlacardText) _returnvalue))

(fn ConstructionScript
  (bind _2dimage (Variables|Image|Get2DImage))
  (|CallParentFunction)
  ;[1 1 1] takes in a user defined image on an actor to actor basis, and places the defined image as the texture. lighting material allows for unlit/lit versions
  (bind _returnvalue (Rendering|Material|CreateDynamicMaterialInstance (Variables|Default|GetArtpieceMesh) 0 (Variables|Image|GetVideoMaterial) "None" :!class /Script/Engine.PrimitiveComponent))
  (Rendering|Material|SetTextureParameterValue _returnvalue "TextureFor2D" (Variables|Image|Get2DImage))
  ;[1 1 1] normal map, specular, and ambient occulsion texture inputs (optional)
  (Rendering|Material|SetTextureParameterValue _returnvalue "NormalMapTexture" (Variables|Image|Get2DImageNormal))
  (Rendering|Material|SetTextureParameterValue _returnvalue "SpecularTexture" (Variables|Image|Get2DImageSpecular))
  (Rendering|Material|SetTextureParameterValue _returnvalue "AmbientOcclusionTexture" (Variables|Image|Get2DImageAmbientOcc))
  ;[1 1 1] calculate scale based on texture aspect ratio
  (Transformation|SetRelativeScale3D (Variables|Default|GetArtpieceMesh) (Math|Vector|MakeVector 1.0 (/ (Math|Conversions|ToFloat(Integer) (Class|MediaTexture|GetHeight _2dimage)) (Math|Conversions|ToFloat(Integer) (Class|MediaTexture|GetWidth _2dimage))) 1.0)))