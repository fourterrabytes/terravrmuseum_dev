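; Interactable door Blueprint that moves the player between the arcade levels.
; Its Interact function plays a 2D button-click sound, then switches on DoorToID to pick the inside, outside or B1 arcade level and opens it by object reference.
; The function returns InteractedWith as false, and the event graph holds only disabled stubs.
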(event EventBeginPlay
  (|CallParentFunction) ; This node is disabled and will not be called.\nDrag off pins to build functionality.
)

(event Collision|EventActorBeginOverlap
  (params (OtherActor :type Actor%20Object%20Reference))
  (|CallParentFunction OtherActor) ; This node is disabled and will not be called.\nDrag off pins to build functionality.
)

(event EventTick
  (params (DeltaSeconds :type Float%20%28single-precision%29))
  (|CallParentFunction DeltaSeconds) ; This node is disabled and will not be called.\nDrag off pins to build functionality.
)

(fn ConstructionScript
  (|CallParentFunction))

(fn Interact
  (params (InteractingActor :type Character%20Object%20Reference))
  (Audio|PlaySound2D "/Engine/VREditor/Sounds/UI/Click_on_Button.Click_on_Button" 1.0 1.0 0.0 0 0)
  (switch int (Variables|Default|GetdoorToID)
    (:0
      (Variables|Default|SetLevel "/Game/ThirdPerson/Maps/insideArcade.insideArcade"))
    (:1
      (Variables|Default|SetLevel "/Game/ThirdPerson/Maps/OutsideArcade.OutsideArcade"))
    (:2
      (Variables|Default|SetLevel "/Game/ThirdPerson/Maps/insideArcade_B1.insideArcade_B1")))
  (Game|OpenLevel(byObjectReference) (Variables|Default|GetLevel))
  (return false 0))