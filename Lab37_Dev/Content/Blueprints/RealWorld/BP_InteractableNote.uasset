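; BP_InteractableNote is an interactable real-world note that shows its text on screen when an actor interacts with it.
; Interact creates an InteractableDialogueUI widget for player controller 0, adds it to the viewport and fills its text box from TextValues, set per instance in the editor.
; If a widget reference is already valid, Interact only clears that reference, without removing the widget from the viewport.
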(event EventBeginPlay)

(event Collision|EventActorBeginOverlap
  (params (OtherActor :type Actor%20Object%20Reference)))

(event EventTick
  (params (DeltaSeconds :type Float%20%28single-precision%29)))

(fn ConstructionScript)

(fn Interact
  (params (InteractingActor :type Character%20Object%20Reference))
  (Utilities|IsValid (Variables|Default|GetdialogueUI)
    (:Is%20Valid
      (Variables|Default|SetdialogueUI 0))
    (:Is%20Not%20Valid
      (bind _returnvalue (UserInterface|CreateWidget "/Game/UIUX/GeneralUI/InteractableDialogueUI.InteractableDialogueUI_C" (Game|GetPlayerController 0)))
      (Variables|Default|SetdialogueUI _returnvalue)
      (UserInterface|Viewport|AddtoViewport _returnvalue 0)
      ;[1 1 1] define on the interactable itself in the editor
      (Rendering|Components|TextRender|SetText (Variables|/Game/UIUX/GeneralUI/InteractableDialogueUI.InteractableDialogueUI_C|GetDialogueTextBox _returnvalue) (Variables|Default|GettextValues))
      (return false 0))))