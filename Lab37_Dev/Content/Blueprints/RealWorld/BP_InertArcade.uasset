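; BP_InertArcade is a construction-time placement actor that lines up copies of a chosen mesh along a spline, presumably as non-interactive arcade dressing.
; The Construction Script fills an InstancedStaticMesh at even intervals, deriving spacing from the mesh's bounding-box X size plus an offset and count from spline length.
; Instances share a fixed local rotation rather than following the spline's direction.
; The event graph has no active runtime logic.
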(event EventBeginPlay
  (|CallParentFunction) ; This node is disabled and will not be called.\nDrag off pins to build functionality.
)

(event Collision|EventActorBeginOverlap
  (params (OtherActor :type Actor%20Object%20Reference))
  (|CallParentFunction OtherActor) ; This node is disabled and will not be called.\nDrag off pins to build functionality.
)

(event EventTick
  (params (DeltaSeconds :type Float%20%28single-precision%29))
  (|CallParentFunction DeltaSeconds) ; This node is disabled and will not be called.\nDrag off pins to build functionality.
)

(fn ConstructionScript
  (bind _placedmesh (Variables|Default|GetPlacedMesh))
  (bind _returnvalue (StaticMesh|GetBoundingBox _placedmesh))
  (bind (_min _max) (Utilities|Struct|BreakBox _returnvalue))
  (Components|StaticMesh|SetStaticMesh (Variables|Default|GetInstancedStaticMesh) (Variables|Default|GetPlacedMesh))
  (bind _output_get (Variables|Default|Setspacing (+ (.X (Math|Vector|BreakVector (- _max _min))) (Variables|Default|Getoffset))))
  (bind _output_get_2 (LocalVariables|SetNumberOfInstances (Math|Float|Floor (/ (Spline|GetSplineLength (Variables|Default|GetSpline)) _output_get))))
  (for _index (range 0 _output_get_2)
    (Components|InstancedStaticMesh|AddInstance (Variables|Default|GetInstancedStaticMesh) (Math|Transform|MakeTransform (Spline|GetLocationatDistanceAlongSpline (Variables|Default|GetSpline) (* _index (Variables|Default|Getspacing)) "Local") "0.000000,90.000000,0.000000") false)))