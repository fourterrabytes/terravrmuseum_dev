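; BP_EMcabinet is an interactable EM machine cabinet that opens its start UI once the power is on.
; A bound power-on event sets the screen's emissive material and raises its rect light intensity.
; Interact checks PowerOn on BPEM_devGameMode, then shows either EM_StartUI or a five-second Eleanor dialogue hinting at a nearby switch.
; The dialogue is skipped if a DialogueBoxUI is already showing.
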(event Custom|addDialogue_PowerOff
  (bind _foundwidgets (Widget|GetAllWidgetsOfClass "/Game/UIUX/GeneralUI/DialogueBoxUI.DialogueBoxUI_C" true))
  (Utilities|IsValid (Utilities|Array|Get(acopy) _foundwidgets)
    (:Is%20Not%20Valid
      (bind _returnvalue (UserInterface|CreateWidget "/Game/UIUX/GeneralUI/DialogueBoxUI.DialogueBoxUI_C" (Game|GetPlayerController 0)))
      (Rendering|Components|TextRender|SetText (Variables|/Game/UIUX/GeneralUI/DialogueBoxUI.DialogueBoxUI_C|GetDialogueTextBox _returnvalue) "Seems like the power isn't on. There should be a power switch nearby...")
      (Rendering|Components|TextRender|SetText (Variables|/Game/UIUX/GeneralUI/DialogueBoxUI.DialogueBoxUI_C|GetNameText _returnvalue) "Eleanor")
      (UserInterface|Viewport|AddtoViewport _returnvalue 0)
      (Utilities|FlowControl|Delay 5.0)
      (Widget|RemovefromParent _returnvalue))))

(event Custom|SetMaterialsPower
  (bind _rectlight (Variables|Default|GetRectLight))
  (Rendering|Material|SetMaterial (Variables|Default|Getscreen) 0 "/Game/Materials/TextureMaterials/EmissiveBase_EMMachine.EmissiveBase_EMMachine")
  (Rendering|Components|Light|SetIntensity _rectlight 1e+04)
  (Development|PrintString (Utilities|String|ToString(Float) (Variables|/Script/Engine.LightComponentBase|GetIntensity _rectlight))))

(event EventBeginPlay
  (EventDispatchers|BindEventtoSetMaterialsAfterPoweron (delegate Custom|SetMaterialsPower)))

(event Collision|EventActorBeginOverlap
  (params (OtherActor :type Actor%20Object%20Reference)))

(event EventTick
  (params (DeltaSeconds :type Float%20%28single-precision%29)))

(fn ConstructionScript)

(fn Interact
  (params (InteractingActor :type Character%20Object%20Reference))
  (bind _asbpem_dev_game_mode (Utilities|Casting|CastToBPEM_devGameMode (Game|GetGameMode)))
  (if (Variables|/Game/BPEM_devGameMode.BPEM_devGameMode_C|GetpowerOn? _asbpem_dev_game_mode)
    (bind _returnvalue (UserInterface|CreateWidget "/Game/UIUX/GeneralUI/EM_StartUI.EM_StartUI_C" (Game|GetPlayerController 0)))
    (UserInterface|Viewport|AddtoViewport _returnvalue 0)
    (else
      (CallFunction|AddDialoguePowerOff)))
  (return false 0))