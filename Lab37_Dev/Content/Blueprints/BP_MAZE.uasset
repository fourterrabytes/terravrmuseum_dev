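; Maze actor that builds a new random maze each time play begins, using an inherited or external UpdateMaze routine.
; BeginPlay calls RandomizeMaze, which picks a random Seed and rebuilds, then prints the seed on screen.
; Optional randomization of size (forced odd), algorithm and path endpoints is present but disconnected, so only the seed varies.
; AddExitNode just moves ExitNode to the world origin and is not called here.
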(event EventBeginPlay
  (CallFunction|RandomizeMaze)
  (Development|PrintString (Utilities|String|ToString(Integer) (Variables|Default|GetSeed)) true true "(R=0.000000,G=0.660000,B=1.000000,A=1.000000)" 1e+01))

(event Collision|EventActorBeginOverlap
  (params (OtherActor :type Actor%20Object%20Reference)))

(event EventTick
  (params (DeltaSeconds :type Float%20%28single-precision%29)))

(fn ConstructionScript)

(fn AddExitNode
  (Transformation|SetWorldLocation (Variables|Default|GetexitNode) "0, 0, 0" false false))

(fn RandomizeMaze
  (Variables|Default|SetSeed (Math|Random|RandomIntegerinRange -1000 1000))
  (Class|Maze|UpdateMaze))